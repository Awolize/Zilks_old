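; AI controller for AITest units that picks enemy units as targets through AI perception and runs AITestBehaviorTree.
; Perception updates feed UpdateStimuli, which, with no valid target, stores a sensed unit of another TeamTag in TargetedUnit and the matching Blackboard key.
; Losing sight of that target clears only the Blackboard key, not the cached variable.
; Allies, buildings and other sightings only print debug messages.
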(event OnTargetPerceptionUpdated(AIPerception)
  (params (Actor :type Actor%20Object%20Reference) (Stimulus :type AI%20Stimulus%20Structure))
  ;[1 1 1] Updated Stimuli
  (CallFunction|UpdateStimuli Actor Stimulus))

(event EventBeginPlay
  ;[1 1 1] Init
  (AI|RunBehaviorTree "/Game/Blueprints/UnitAI/AITestBehaviorTree.AITestBehaviorTree"))

(event EventPossess
  (params (PossessedPawn :type Pawn%20Object%20Reference))
  (bind _asaitest (Utilities|Casting|CastToAITest (Pawn|GetControlledPawn)))
  (Variables|Default|SetControlledUnit _asaitest))

(fn ConstructionScript)

(fn UpdateStimuli
  (params (Actor :type Actor%20Object%20Reference) (Stimulus :type AI%20Stimulus%20Structure))
  (LocalVariables|Set_Actor Actor)
  (LocalVariables|Set_Stimuli Stimulus)
  (Utilities|IsValid (Variables|Default|GetTargetedUnit)
    (:Is%20Valid
      (if (== (Variables|Default|GetTargetedUnit) (LocalVariables|Get_Actor))
        (if (.bSuccessfullySensed (Utilities|Struct|BreakAIStimulus (LocalVariables|Get_Stimuli)))
          (Development|PrintString "AITestCtr - Targeted Unit seen again" true true "(R=1.000000,G=0.016606,B=0.000000,A=1.000000)")
          (else
            (AI|Components|Blackboard|ClearValue (AI|GetBlackboard 0) (Utilities|Name|MakeLiteralName "TargetedUnit"))))
        (else
          (Development|PrintString "AITestCtr - New enemy within range"))))
    (:Is%20Not%20Valid
      ;[1 1 1] Sensed actor is a valid Unit?
      (bind _asaitest (Utilities|Casting|CastToAITest (LocalVariables|Get_Actor))
        (:then
          (LocalVariables|Set_Unit _asaitest)
          ;[1 1 1] Sensed Unit NOT same team as us?
          (if (!= (Variables|/Game/Blueprints/UnitAI/AITest.AITest_C|GetTeamTag (LocalVariables|Get_Unit)) (Variables|/Game/Blueprints/UnitAI/AITest.AITest_C|GetTeamTag (Variables|Default|GetControlledUnit)))
            ;[1 1 1] Set Unit as TargetedUnit
            (bind _output_get (Variables|Default|SetTargetedUnit (LocalVariables|Get_Unit)))
            (AI|Components|Blackboard|SetValueasObject (AI|GetBlackboard 0) (Utilities|Name|MakeLiteralName "TargetedUnit") _output_get)
            (else
              (Development|PrintString "AITestCtr - New ally within range"))))
        (:CastFailed
          (Utilities|Casting|CastToBuilding (LocalVariables|Get_Actor)
            (:then
              (Development|PrintString "Building is new target")
              (Utilities|Casting|CastToBuilding_Base (LocalVariables|Get_Actor)
                (:then
                  (Development|PrintString "Building is a Base"))
                (:CastFailed
                  (Development|PrintString "Building is a Turret"))))
            (:CastFailed
              (Development|PrintString "Could not cast to building"))))))))