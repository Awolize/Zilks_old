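; Behavior Tree task that lets an AI unit damage the target stored under its TargetedUnit blackboard key.
; It casts the target to AITest or Building and applies point damage along the pawn's forward vector, using UnitDamage for AITest and a separate BaseDamage for Building.
; The task succeeds after dealing damage; any other target prints an error and fails it.
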(event EventReceiveExecuteAI
  (params (OwnerController :type AI%20Controller%20Object%20Reference) (ControlledPawn :type Pawn%20Object%20Reference))
  (bind _returnvalue (Transformation|GetActorForwardVector ControlledPawn))
  (bind _returnvalue_2 (Collision|MakeHitResult false false 0.0 0.0 "0, 0, 0" "0, 0, 0" "0,0,1" "0,0,1" 0 0))
  (bind _targetedunit (Variables|Default|GetTargetedUnit))
  (bind _returnvalue_3 (Class|BTFunctionLibrary|GetBlackboardValueasObject _targetedunit))
  (bind _asaitest (Utilities|Casting|CastToAITest _returnvalue_3)
    (:then
      (Game|Damage|ApplyPointDamage _asaitest (Variables|Default|GetUnitDamage) _returnvalue _returnvalue_2 OwnerController 0 "/Script/Engine.DamageType")
      (AI|BehaviorTree|FinishExecute true))
    (:CastFailed
      (bind _asbuilding (Utilities|Casting|CastToBuilding _returnvalue_3)
        (:then
          (Game|Damage|ApplyPointDamage _asbuilding (Variables|Default|GetBaseDamage) _returnvalue _returnvalue_2 OwnerController 0 "/Script/Engine.DamageType")
          (AI|BehaviorTree|FinishExecute true))
        (:CastFailed
          (Development|PrintString "DealDamage - Error Unknown object" true true "(R=1.000000,G=0.000000,B=0.017848,A=1.000000)")
          (AI|BehaviorTree|FinishExecute false))))))