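; GetTile is a unit AI behavior tree task that writes the controlled pawn's current grid tile to the blackboard.
; It fetches the grid through ZilksGameModeNew and converts the pawn's world location into a tile row and column.
; A valid tile is stored in the Row and Column keys and the task succeeds; otherwise it fails and prints an outside-grid warning.
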(event EventReceiveExecuteAI
  (params (OwnerController :type AI%20Controller%20Object%20Reference) (ControlledPawn :type Pawn%20Object%20Reference))
  (Variables|Default|SetLocation (Transformation|GetActorLocation ControlledPawn))
  (bind _grid (CallFunction|GetGrid))
  (Variables|Default|SetGrid _grid)
  (bind (_valid_ _row _column) (Default|LocationtoTile (Variables|Default|GetGrid) (Variables|Default|GetLocation)))
  (if _valid_
    (Variables|Default|Set_Row _row)
    (Variables|Default|Set_Column _column)
    (Class|BTFunctionLibrary|SetBlackboardValueasInt (Variables|Default|GetRow) (Variables|Default|Get_Row))
    (Class|BTFunctionLibrary|SetBlackboardValueasInt (Variables|Default|GetColumn) (Variables|Default|Get_Column))
    (AI|BehaviorTree|FinishExecute true)
    (else
      (AI|BehaviorTree|FinishExecute false)
      (Development|PrintString "GetTile - Outside grid?" true true "(R=1.000000,G=0.018129,B=0.000000,A=1.000000)" 1e+01))))

(fn GetGrid
  (bind _gamemode (Utilities|GetGameMode)
    (:_Exec
      (bind _grid (Default|GetGrid _gamemode))
      (return _grid))))