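; Behavior tree task that picks a unit's next move target on the grid.
; It gets the grid and team from the pawn's owning ZilksPlayerControllerBP, or the first one found in the level for manually spawned units.
; The grid turns the blackboard row and column into the next tile's world location, which is written to NewLocation.
; The task fails when no controller, valid tile or valid location is found.
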(event EventReceiveExecuteAI
  (params (OwnerController :type AI%20Controller%20Object%20Reference) (ControlledPawn :type Pawn%20Object%20Reference))
  (Variables|Default|SetControlled%20Pawn ControlledPawn)
  (bind _aszilks_player_controller_bp (Utilities|Casting|CastToZilksPlayerControllerBP (Components|GetOwner ControlledPawn))
    (:then
      (Variables|Default|SetAs%20Zilks%20Player%20Controller%20BP _aszilks_player_controller_bp)
      (bind _grid (Default|GetGrid (Variables|Default|GetAs%20Zilks%20Player%20Controller%20BP) :!label _label))
      (bind _output_get (Variables|Default|SetGrid _grid))
      (bind (_done_ _valid_ _newrow _newcolumn) (Default|NextTile _output_get (Variables|/Game/Blueprints/ZilksPlayerControllerBP.ZilksPlayerControllerBP_C|GetTeam (Variables|Default|GetAs%20Zilks%20Player%20Controller%20BP)) (Class|BTFunctionLibrary|GetBlackboardValueasInt (Variables|Default|GetRow)) (Class|BTFunctionLibrary|GetBlackboardValueasInt (Variables|Default|GetColumn))))
      (if _valid_
        (bind (_valid__2 _location) (Default|TiletoLocation (Variables|Default|GetGrid) _newrow _newcolumn))
        (Class|BTFunctionLibrary|SetBlackboardValueasBool (Variables|Default|GetNewLocation?) _valid__2)
        (AI|BehaviorTree|SetBlackboardValueasVector (Variables|Default|GetNewLocation) _location)
        (AI|BehaviorTree|FinishExecute _valid__2)
        (else
          (AI|BehaviorTree|FinishExecute false))))
    (:CastFailed
      ;[1 1 1] If Unit has been spawned manually
      (bind _outactors (Actor|GetAllActorsOfClass "/Game/Blueprints/ZilksPlayerControllerBP.ZilksPlayerControllerBP_C"))
      (if (Utilities|Array|IsValidIndex _outactors)
        (Variables|Default|SetAs%20Zilks%20Player%20Controller%20BP (Utilities|Array|Get(acopy) _outactors))
        (goto _label)
        (else
          (Development|PrintString "AIUnit - Owner is NOT the ZilksPlayerControllerBP" true true "(R=1.000000,G=0.000000,B=0.008232,A=1.000000)")
          (AI|BehaviorTree|FinishExecute false))))))