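; Tile grid actor that forms a two-team arena with a base at each end of every column.
; Construction script lays instanced floor, middle border and base-edge meshes from HalfRows, Columns and TileSize.
; BeginPlay uses the IterateTiles macro to find each team's end row, spawning and storing Building_Base actors there.
; Helper functions convert between world and tile coordinates, restrict unit spawning to each team's half, step units forward and look up bases by column.
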(event Custom|InitGame)

(event Custom|StartGame)

(event EventBeginPlay
  (Utilities|Array|Clear (Variables|Default|GetTeamRightBases))
  (Utilities|Array|Clear (Variables|Default|GetTeamLeftBases))
  (Utilities|FlowControl|Sequence
    (:then_0
      (bind _locations (CallFunction|GetTeamBaseLocations "(TagName=\"Team.RightTeam\")"))
      (for _array_element _locations
        (bind _returnvalue (Game|SpawnActorfromClass "/Game/Blueprints/Buildings/Building_Base.Building_Base_C" (Math|Transform|MakeTransform _array_element "0, 0, 0" "2.000000,2.000000,2.000000") "AlwaysSpawn" 0 "(TagName=\"Team.RightTeam\")" 0))
        (Utilities|Array|Add (Variables|Default|GetTeamRightBases) _returnvalue)
        (bind (_valid_ _row _column) (CallFunction|LocationtoTile _array_element))
        (Development|PrintString (Utilities|String|Append "(" (Utilities|String|ToString(Integer) _row) "," (Utilities|String|ToString(Integer) _column) ")"))))
    (:then_1
      (bind _locations_2 (CallFunction|GetTeamBaseLocations "(TagName=\"Team.LeftTeam\")"))
      (for _array_element_2 _locations_2
        (bind _returnvalue_2 (Game|SpawnActorfromClass "/Game/Blueprints/Buildings/Building_Base.Building_Base_C" (Math|Transform|MakeTransform _array_element_2 "0, 0, 0" "2.000000,2.000000,2.000000") "AlwaysSpawn" 0 "(TagName=\"Team.LeftTeam\")" 0))
        (Utilities|Array|Add (Variables|Default|GetTeamLeftBases) _returnvalue_2)
        (bind (_valid__2 _row_2 _column_2) (CallFunction|LocationtoTile _array_element_2))
        (Development|PrintString (Utilities|String|Append "(" (Utilities|String|ToString(Integer) _row_2) "," (Utilities|String|ToString(Integer) _column_2) ")"))))))

(event Collision|EventActorBeginOverlap
  (params (OtherActor :type Actor%20Object%20Reference)))

(event EventTick
  (params (DeltaSeconds :type Float%20%28single-precision%29)))

(fn ConstructionScript
  (bind _halfrows (Variables|Const|GetHalfRows))
  (bind _returnvalue (* _halfrows 2))
  (Utilities|FlowControl|Sequence
    (:then_0
      ;[1 1 1] Generate Arena
      (Variables|Const|SetRows%20%28read%20only%29 (+ _returnvalue 1))
      (for _index (range 0 _returnvalue)
        (LocalVariables|SetColumn _index)
        (for _index_2 (range 0 (- (Variables|Const|GetColumns) 1))
          (LocalVariables|SetRow _index_2)
          (LocalVariables|SetY-Coord (Math|Conversions|ToFloat(Integer) (* (LocalVariables|GetRow) (Variables|Const|GetTileSize))))
          (LocalVariables|SetX-Coord (Math|Conversions|ToFloat(Integer) (* (LocalVariables|GetColumn) (Variables|Const|GetTileSize))))
          (Utilities|FlowControl|Sequence
            (:then_0
              (if (== (LocalVariables|GetColumn) (Variables|Const|GetHalfRows))
                ;;[1 1 1] Middle border
                (Components|InstancedStaticMesh|AddInstance (Variables|Default|GetMiddleBorder) (Math|Transform|MakeTransform (Math|Vector|MakeVector (+ (/ (.x (.Max (Components|StaticMesh|GetLocalBounds (Variables|Default|GetFloor)))) 2.0) (LocalVariables|GetX-Coord)) (LocalVariables|GetY-Coord) 0.0) "0.000000,90.000000,0.000000" "1.000000,1.000000,1.000000") false)))
            (:then_1
              ;;[1 1 1] Floors
              (Components|InstancedStaticMesh|AddInstance (Variables|Default|GetFloor) (Math|Transform|MakeTransform (Math|Vector|MakeVector (LocalVariables|GetX-Coord) (LocalVariables|GetY-Coord) 0.0) "0, 0, 0" "1.000000,1.000000,1.000000") false))
            (:then_2
              (if (== (LocalVariables|GetColumn) 0)
                ;;[1 1 1] Base P1
                (Components|InstancedStaticMesh|AddInstance (Variables|Default|GetBase%20P1) (Math|Transform|MakeTransform (Math|Vector|MakeVector (LocalVariables|GetX-Coord) (LocalVariables|GetY-Coord) 0.0) "0.000000,90.000000,0.000000" "1.000000,1.000000,1.000000") false)))
            (:then_3
              (if (== (LocalVariables|GetColumn) (* (Variables|Const|GetHalfRows) 2))
                ;;[1 1 1] Base P2
                (Components|InstancedStaticMesh|AddInstance (Variables|Default|GetBase%20P2) (Math|Transform|MakeTransform (Math|Vector|MakeVector (+ (LocalVariables|GetX-Coord) (.x (.Max (Components|StaticMesh|GetLocalBounds (Variables|Default|GetFloor))))) (LocalVariables|GetY-Coord) 0.0) "0.000000,90.000000,0.000000" "1.000000,1.000000,1.000000") false)))))))))

(fn LocationtoTile
  (params (HitLocation :type Vector))
  (bind _self self)
  (bind _tilesize (Variables|Const|GetTileSize))
  (bind _tilesize_2 (Variables|Const|GetTileSize))
  (bind _returnvalue (Transformation|GetActorLocation _self))
  (bind _returnvalue_2 (- (.x HitLocation) (.x _returnvalue)))
  (bind _returnvalue_3 (- (.y HitLocation) (.y _returnvalue)))
  (bind _returnvalue_4 (/ _returnvalue_3 _tilesize))
  (bind _returnvalue_5 (/ _returnvalue_2 _tilesize_2))
  (bind _returnvalue_6 (Math|Float|Floor _returnvalue_4))
  (bind _returnvalue_7 (Math|Float|Floor _returnvalue_5))
  (bind _valid_ (CallFunction|ValidTile? _returnvalue_7 _returnvalue_6))
  (return _valid_ _returnvalue_7 _returnvalue_6))

(fn ValidTile?
  (params (Row :type Integer) (Column :type Integer))
  (return (Math|Boolean|ANDBoolean (<= Row (Variables|Const|GetRows%20%28read%20only%29)) (>= Row 0) (>= Column 0) (<= Column (Variables|Const|GetColumns)))))

(fn TiletoLocation
  (params (Row :type Integer) (Column :type Integer))
  (bind _returnvalue (Math|Float|SelectFloat 2.0 0.0 true))
  (bind _self self)
  (bind _tilesize (Variables|Const|GetTileSize))
  (bind _tilesize_2 (Variables|Const|GetTileSize))
  (bind _returnvalue_2 (Transformation|GetActorLocation _self))
  (bind _returnvalue_3 (/ _tilesize _returnvalue))
  (return true (Math|Vector|MakeVector (+ (* Row _tilesize_2) (.x _returnvalue_2) _returnvalue_3) (+ (* Column _tilesize_2) (.y _returnvalue_2) _returnvalue_3) 0.0)))

(fn AllowedSpawnUnit?
  (params (Team :type Gameplay%20Tag%20Structure) (Row :type Integer) (Column :type Integer))
  (LocalVariables|Set_TeamTag Team)
  (LocalVariables|Set_Row Row)
  (LocalVariables|Set_Column Column)
  (bind _valid_ (CallFunction|ValidTile? (LocalVariables|Get_Row) (LocalVariables|Get_Column)))
  (if _valid_
    (if (Math|Boolean|ANDBoolean (== (LocalVariables|Get_TeamTag) "(TagName=\"Team.RightTeam\")") (< (LocalVariables|Get_Row) (Variables|Const|GetHalfRows)) (<= (LocalVariables|Get_Column) (Variables|Const|GetColumns)))
      (return true)
      (elif (Math|Boolean|ANDBoolean (== (LocalVariables|Get_TeamTag) "(TagName=\"Team.LeftTeam\")") (> (LocalVariables|Get_Row) (Variables|Const|GetHalfRows)) (<= (LocalVariables|Get_Column) (Variables|Const|GetColumns)))
        (return true)
        (else
          ;[1 1 1] Else
          (Development|PrintText "TileGridBP - Invalid move")
          (return false))))
    (else
      (return false))))

(fn NextTile
  (params (Team :type Gameplay%20Tag%20Structure) (Row :type Integer) (Column :type Integer))
  ;[1 1 1] Basic Check
  (LocalVariables|Set_Team Team)
  (LocalVariables|Set_Row Row)
  (LocalVariables|Set_Column Column)
  (bind _valid_ (CallFunction|ValidTile? Row Column))
  (if (and _valid_ (or (== (LocalVariables|Get_Team) "(TagName=\"Team.LeftTeam\")") (== (LocalVariables|Get_Team) "(TagName=\"Team.RightTeam\")")))
    (bind _valid__2 (CallFunction|ValidTile? (+ (LocalVariables|Get_Row) (Math|Integer|SelectInt 1 -1 (== (LocalVariables|Get_Team) "(TagName=\"Team.RightTeam\")"))) (LocalVariables|Get_Column)))
    (if _valid__2
      (return false true (+ (LocalVariables|Get_Row) (Math|Integer|SelectInt 1 -1 (== (LocalVariables|Get_Team) "(TagName=\"Team.RightTeam\")"))) (LocalVariables|Get_Column))
      (else
        (return true false (LocalVariables|Get_Row) (LocalVariables|Get_Column))))
    (else
      (return false false -1 -1))))

(fn GetTeamBaseLocations
  (params (Team :type Gameplay%20Tag%20Structure))
  (bind (_row _column) (Utilities|IterateTiles)
    (:LoopBody
      (if (== _row (Math|Integer|SelectInt 0 (- (Variables|Const|GetRows%20%28read%20only%29) 1) (== Team "(TagName=\"Team.RightTeam\")")))
        (bind _location (CallFunction|TiletoLocation _row _column))
        (Utilities|Array|Add (LocalVariables|GetResultVector) _location)))
    (:Completed
      (return (LocalVariables|GetResultVector)))))

(fn GetTeamBase
  (params (ToFindTeam :type Gameplay%20Tag%20Structure) (Column :type Integer))
  (bind _teamrightbases (Variables|Default|GetTeamRightBases))
  (bind _teamleftbases (Variables|Default|GetTeamLeftBases))
  (if (== ToFindTeam "(TagName=\"Team.RightTeam\")")
    (return (Utilities|Array|IsValidIndex _teamrightbases Column) (Utilities|Array|Get(acopy) _teamrightbases Column))
    (else
      (return (Utilities|Array|IsValidIndex _teamleftbases Column) (Utilities|Array|Get(acopy) _teamleftbases Column)))))