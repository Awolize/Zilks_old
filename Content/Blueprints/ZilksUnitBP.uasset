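; ZilksUnitBP is a unit actor that snaps itself onto the center or position of a tile in a TileGridBP grid.
; SetGrid caches the first TileGridBP found in the level and prints whether it is valid.
; The construction script converts the actor's location to a tile and back to snap it in the editor.
; BeginPlay repeats the snap and destroys the unit if no grid or valid tile is found.
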(event EventBeginPlay
  (bind _grid (Variables|Default|GetGrid))
  (bind _returnvalue (CallFunction|SetGrid))
  (if _returnvalue
    (bind (_valid_ _row _column) (Default|LocationtoTile _grid (Transformation|GetActorLocation)))
    (if _valid_
      (bind _location (Default|TiletoLocation _grid _row _column))
      (Transformation|SetActorLocation _location false true)
      (else
        (Actor|DestroyActor :!label _label)))
    (else
      (goto _label))))

(event Collision|EventActorBeginOverlap
  (params (OtherActor :type Actor%20Object%20Reference)))

(event EventTick
  (params (DeltaSeconds :type Float%20%28single-precision%29)))

(fn ConstructionScript
  (bind _grid (Variables|Default|GetGrid))
  (bind _returnvalue (CallFunction|SetGrid))
  (if _returnvalue
    (bind (_valid_ _row _column) (Default|LocationtoTile _grid (Transformation|GetActorLocation)))
    (if _valid_
      (bind _location (Default|TiletoLocation _grid _row _column))
      (Transformation|SetActorLocation _location false true))))

(fn SetGrid
  (bind _outactors (Actor|GetAllActorsOfClass "/Game/Blueprints/TileGridBP.TileGridBP_C"))
  (if (Utilities|Array|IsValidIndex _outactors)
    (Variables|Default|SetGrid (Utilities|Array|Get(acopy) _outactors))
    (Development|PrintText "ZilksUnitBP: valid Grid" true true "(R=0.000000,G=1.000000,B=0.000000,A=1.000000)")
    (return (Utilities|Array|IsValidIndex _outactors))
    (else
      (Development|PrintText "ZilksUnitBP: invalid Grid" true true "(R=1.000000,G=0.000000,B=0.000000,A=1.000000)"))))