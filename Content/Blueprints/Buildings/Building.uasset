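; Building actor that snaps to the game's tile grid and can be destroyed by damage.
; On BeginPlay it fetches the grid from ZilksGameModeNew, then teleports to the center of its tile, destroying itself if the grid or tile is invalid.
; The construction script adds a team gameplay tag.
; Point damage lowers Health, printing debug messages and destroying the actor at zero.
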(event EventBeginPlay
  (bind _grid (CallFunction|GetGrid))
  (bind _output_get (Variables|Private|SetGrid _grid))
  (if (Utilities|IsValid _output_get)
    (CallFunction|TeleporttoMiddleOfTile)
    (else
      (Development|PrintString "Grid Not valid")
      (Actor|DestroyActor))))

(event Collision|EventActorBeginOverlap
  (params (OtherActor :type Actor%20Object%20Reference)))

(event EventTick
  (params (DeltaSeconds :type Float%20%28single-precision%29)))

(event Game|Damage|EventPointDamage
  (params (Damage :type Float%20%28single-precision%29) (DamageType :type Damage%20Type%20Object%20Reference) (HitLocation :type Vector :default "0, 0, 0") (HitNormal :type Vector :default "0, 0, 0") (HitComponent :type Primitive%20Component%20Object%20Reference) (BoneName :type Name :default "None") (ShotFromDirection :type Vector :default "0, 0, 0") (InstigatedBy :type Controller%20Object%20Reference) (DamageCauser :type Actor%20Object%20Reference) (HitInfo :type Hit%20Result%20Structure%20%28by%20ref%29))
  (bind _output_get (Variables|Default|SetHealth (- (Variables|Default|GetHealth) Damage)))
  (if (<= _output_get 0.0)
    (Actor|DestroyActor)
    (Development|PrintString "Building Destroyed")
    (else
      (Development|PrintString (Utilities|String|Append "Health: " (Utilities|String|ToString(Float) (Variables|Default|GetHealth)))))))

(fn ConstructionScript
  (GameplayTags|AddGameplayTag (Variables|Default|GetActorTagContainer) (Variables|Default|GetTeamTag) :!class /Script/GameplayTags.BlueprintGameplayTagLibrary)
  (Development|PrintString "Setting team test" true true "(R=1.000000,G=0.000000,B=0.995059,A=1.000000)" 1e+01))

(fn GetGrid
  (bind _gamemode (Utilities|GetGameMode)
    (:_Exec
      (bind _grid (Default|GetGrid _gamemode))
      (return _grid))))

(fn TeleporttoMiddleOfTile
  (bind (_valid_ _row _column) (Default|LocationtoTile (Variables|Private|GetGrid) (Transformation|GetActorLocation)))
  (if _valid_
    (bind _location (Default|TiletoLocation (Variables|Private|GetGrid) _row _column))
    (Transformation|SetActorLocation _location false true)
    (else
      (Actor|DestroyActor))))