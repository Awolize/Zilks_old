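; ZilksGameModeNew is a game mode Blueprint that holds a reference to the level's TileGridBP actor.
; On BeginPlay, SetGrid searches for TileGridBP actors, stores the first one as Grid and reports success, with debug prints for either outcome.
; GetGrid exposes the cached reference to other code.
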(event EventBeginPlay
  (bind _returnvalue (CallFunction|SetGrid))
  (if _returnvalue
    (Development|PrintString "GAMEMODE - Grid set" true true "(R=0.000000,G=1.000000,B=0.140301,A=1.000000)")
    (else
      (Development|PrintString "GAMEMODE - Grid NOT set" true true "(R=1.000000,G=0.009182,B=0.000000,A=1.000000)"))))

(event EventTick
  (params (DeltaSeconds :type Float%20%28single-precision%29)))

(fn ConstructionScript)

(fn SetGrid
  (bind _outactors (Actor|GetAllActorsOfClass "/Game/Blueprints/TileGridBP.TileGridBP_C"))
  (if (Utilities|Array|IsValidIndex _outactors)
    (Variables|Default|SetGrid (Utilities|Array|Get(acopy) _outactors))
    (Development|PrintText "ZilksGameModeNew: valid Grid" true true "(R=0.000000,G=1.000000,B=0.000000,A=1.000000)")
    (return (Utilities|Array|IsValidIndex _outactors))
    (else
      (Development|PrintText "ZilksGameModeNew: invalid Grid" true true "(R=1.000000,G=0.000000,B=0.000000,A=1.000000)"))))

(fn GetGrid
  (return (Variables|Default|GetGrid)))