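; BP_ZilksGridCharacter is a player character that turns the mouse cursor position into a selected tile on a BP_ZilksGrid.
; Each tick it traces under the cursor, aligns CursorToWorld to the hit and converts that location to a row and column.
; It passes the tile to BP_ZilksPlayerController, or -1/-1 on a miss.
; It also finds the grid, handles yaw-relative sideways movement and adds a team gameplay tag on construction.
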(event EventTick
  (params (DeltaSeconds :type Float%20%28single-precision%29))
  (Utilities|IsValid (Variables|Private|GetGrid)
    (:Is%20Valid
      (CallFunction|UpdateCursorPosition))
    (:Is%20Not%20Valid
      (bind _grid (CallFunction|GetGrid))
      (Variables|Private|SetGrid _grid))))

(event EventBeginPlay
  (bind _grid (CallFunction|GetGrid))
  (Variables|Private|SetGrid _grid))

(event Input|AxisEvents|InputAxisMoveRight
  (params (AxisValue :type Float%20%28single-precision%29))
  (Pawn|Input|AddMovementInput (Math|Vector|GetRightVector (Math|Rotator|MakeRotator 0.0 0.0 (.Yaw (Math|Rotator|BreakRotator (Pawn|GetControlRotation :!class /Script/Engine.Pawn))))) AxisValue false))

(fn ConstructionScript
  (GameplayTags|AddGameplayTag (Variables|Default|GetActorTagContainer) (Variables|Default|GetTeamTag) :!class /Script/GameplayTags.BlueprintGameplayTagLibrary))

(fn UpdateCursorPosition
  (bind _returnvalue (Pawn|GetController))
  (bind _asplayer_controller (Utilities|Casting|CastToPlayerController _returnvalue))
  (bind (_hitresult _returnvalue_2) (Game|Player|GetHitResultUnderCursorbyChannel _asplayer_controller "TraceTypeQuery1" true))
  (bind (_bblockinghit _binitialoverlap _time _distance _location _impactpoint _normal _impactnormal) (Collision|BreakHitResult _hitresult))
  (if _returnvalue_2
    (bind _output_get (LocalVariables|SetHitLocation _location))
    (Transformation|SetWorldLocationAndRotation (Variables|Default|GetCursorToWorld) _output_get (Math|Rotator|MakeRotationfromAxes _impactnormal "0, 0, 0" "0, 0, 0") false false)
    (bind (_valid_ _row _column) (Default|LocationtoTile (Variables|Private|GetGrid) (LocalVariables|GetHitLocation)))
    (bind _asbp_zilks_player_controller (Utilities|Casting|CastToBP_ZilksPlayerController (Game|GetPlayerController 0)))
    (Default|SetSelectedTile _asbp_zilks_player_controller _row _column)
    (else
      (bind _asbp_zilks_player_controller_2 (Utilities|Casting|CastToBP_ZilksPlayerController (Pawn|GetController)))
      (Default|SetSelectedTile _asbp_zilks_player_controller_2 -1 -1))))

(fn GetGrid
  (bind _outactors (Actor|GetAllActorsOfClass "/Game/ZilksBP/BP_ZilksGrid.BP_ZilksGrid_C"))
  (return (Utilities|Array|Get(acopy) _outactors)))