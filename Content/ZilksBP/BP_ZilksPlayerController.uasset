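; Player controller for a grid-based, team unit-spawning game where money buys AI units on tiles.
; SetSelectedTile validates a tile and moves the pawn's floor highlight onto it.
; Clicking SetDestination deducts money locally, ignoring its tile check, then calls a server spawn event that checks tile and team before spawning a team-tagged AI with a behavior tree.
; A looping timer adds income, marked to move to the game mode.
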(event Custom|GenerateMoney
  ;[1 1 1] Money gen - Move to game mode together with buying units
  (if true
    (bind _output_get (Variables|Default|SetMoney (+ (Variables|Default|GetMoney) 1e+01)))
    (Development|PrintString (Utilities|String|ToString(Float) _output_get) true true "(R=1.000000,G=0.795439,B=0.000000,A=1.000000)" 5.0)))

(event Custom|Spawn%20Entity%20on%20Server
  (params (SelectedRow :type Integer) (SelectedColumn :type Integer) (AIToSpawn :type Pawn%20Class%20Reference) (TeamTag1 :type Gameplay%20Tag%20Structure))
  (bind _valid_ (Default|ValidTile? (Variables|Private|GetGrid) SelectedRow SelectedColumn))
  (if _valid_
    (CallFunction|SpawnUnit AIToSpawn SelectedRow SelectedColumn TeamTag1)
    (Development|PrintString "Hello")))

(event EventBeginPlay
  (CallFunction|GetGrid)
  (Variables|Default|SetbShowMouseCursor true)
  (Utilities|Time|SetTimerbyEvent (delegate Custom|GenerateMoney) 5.0 true))

(event EventPossess
  (params (PossessedPawn :type Pawn%20Object%20Reference))
  (bind _asbp_zilks_grid_character (Utilities|Casting|CastToBP_ZilksGridCharacter PossessedPawn))
  (Development|SetHiddeninGame (Variables|/Game/ZilksBP/BP_ZilksGridCharacter.BP_ZilksGridCharacter_C|GetSelectedFloor _asbp_zilks_grid_character) false false))

(event Input|ActionEvents|InputActionSetDestination
  (params (Key :type Key%20Structure :default "None"))
  (bind _selectedcolumn (Variables|Default|GetSelectedColumn))
  (bind _selectedrow (Variables|Default|GetSelectedRow))
  (:Pressed
    (Utilities|IsValid (Variables|Private|GetGrid)
      (:Is%20Valid
        (bind _asbp_zilks_grid_character (Utilities|Casting|CastToBP_ZilksGridCharacter (Pawn|GetControlledPawn)))
        (Default|ValidTile? (Variables|Private|GetGrid) _selectedrow _selectedcolumn)
        (if true
          (if (>= (- (Variables|Default|GetMoney) 1e+01) 0.0)
            (Variables|Default|SetMoney (- (Variables|Default|GetMoney) 1e+01))
            (CallFunction|SpawnEntityonServer _selectedrow _selectedcolumn "/Game/ZilksBP/UnitAI/AITest.AITest_C" (Variables|/Game/ZilksBP/BP_ZilksGridCharacter.BP_ZilksGridCharacter_C|GetTeamTag _asbp_zilks_grid_character)))
          (else
            (Development|PrintString "Invalid move, handled on client")))))))

(fn ConstructionScript)

(fn SetSelectedTile
  (params (Row :type Integer) (Column :type Integer))
  (bind _returnvalue (Game|Player|GetPlayerPawn 0))
  (bind _returnvalue_2 (Game|Player|GetPlayerPawn 0))
  (bind _grid (Variables|Private|GetGrid))
  (bind _grid_2 (Variables|Private|GetGrid))
  (bind _returnvalue_3 (Transformation|GetActorLocation _grid_2))
  (bind _asbp_zilks_grid_character (Utilities|Casting|CastToBP_ZilksGridCharacter _returnvalue))
  (bind _asbp_zilks_grid_character_2 (Utilities|Casting|CastToBP_ZilksGridCharacter _returnvalue_2))
  (bind _tilesize (Variables|/Game/ZilksBP/BP_ZilksGrid.BP_ZilksGrid_C|GetTileSize _grid))
  (bind _selectedfloor (Variables|/Game/ZilksBP/BP_ZilksGridCharacter.BP_ZilksGridCharacter_C|GetSelectedFloor _asbp_zilks_grid_character))
  (bind _selectedfloor_2 (Variables|/Game/ZilksBP/BP_ZilksGridCharacter.BP_ZilksGridCharacter_C|GetSelectedFloor _asbp_zilks_grid_character_2))
  (Utilities|GridValid?)
  (LocalVariables|Set_Rows Row)
  (LocalVariables|Set_Column Column)
  (bind _valid_ (Default|ValidTile? (Variables|Private|GetGrid) (LocalVariables|Get_Rows) (LocalVariables|Get_Column)))
  (if _valid_
    (Variables|Default|SetSelectedRow (LocalVariables|Get_Rows))
    (Variables|Default|SetSelectedColumn (LocalVariables|Get_Column))
    ;[1 1 1] Show Selected Tile
    (Transformation|SetWorldLocation _selectedfloor (Math|Vector|MakeVector (+ (Math|Conversions|ToFloat(Integer) (* (LocalVariables|Get_Rows) _tilesize)) (.x _returnvalue_3) 2e+02) (+ (Math|Conversions|ToFloat(Integer) (* _tilesize (LocalVariables|Get_Column))) (.y _returnvalue_3) 2e+02) 1e+01) false true)
    (Rendering|SetVisibility _selectedfloor true false)
    (else
      (Variables|Default|SetSelectedRow -1)
      (Variables|Default|SetSelectedColumn -1)
      ;[1 1 1] Hide Selected Tile
      (Transformation|SetWorldLocation _selectedfloor_2 (Math|Vector|MakeVector 0.0 0.0 1e+01) false true)
      (Rendering|SetVisibility _selectedfloor_2 false false))))

(fn SpawnUnit
  (params (AIToSpawn :type Pawn%20Class%20Reference) (Row :type Integer) (Column :type Integer) (TeamTag1 :type Gameplay%20Tag%20Structure))
  (bind _grid (Variables|Private|GetGrid))
  (Utilities|GridValid?)
  (bind _output_get (LocalVariables|SetTeamTag TeamTag1))
  (bind _valid_ (Default|AllowedSpawnUnit? _grid _output_get Row Column))
  (if _valid_
    (bind (_valid__2 _location) (Default|TiletoLocation _grid Row Column))
    (if _valid__2
      (bind _returnvalue (AI|SpawnAIFromClass AIToSpawn "/Game/ZilksBP/UnitAI/AITestBehaviorTree.AITestBehaviorTree" _location "0, 0, 0" true self))
      (bind _asaitest (Utilities|Casting|CastToAITest _returnvalue))
      (Variables|/Game/ZilksBP/UnitAI/AITest.AITest_C|SetTeamTag _asaitest (LocalVariables|GetTeamTag))
      (return true)
      (else
        _)))
  (return false))

(fn GetGrid
  (bind _outactors (Actor|GetAllActorsOfClass "/Game/ZilksBP/BP_ZilksGrid.BP_ZilksGrid_C"))
  (Utilities|IsValid (Utilities|Array|Get(acopy) _outactors)
    (:Is%20Valid
      (return (Utilities|Array|Get(acopy) _outactors) true))
    (:Is%20Not%20Valid
      (return 0 false))))

(fn SetGrid
  (params (Grid :type BP%20Zilks%20Grid%20Object%20Reference))
  (Variables|Private|SetGrid Grid)
  (return))

(fn UpdateGrid
  (bind (_grid _valid_) (CallFunction|GetGrid))
  (if _valid_
    (CallFunction|SetGrid _grid)
    (return true)
    (else
      (return false))))