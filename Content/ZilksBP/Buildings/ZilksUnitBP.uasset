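; ZilksUnitBP is a unit actor that snaps itself to the centralized tile grid supplied by BP_ZilksGameMode.
; The construction script and BeginPlay both convert its location to a tile and back to align it.
; At BeginPlay it destroys itself if the grid is missing or the tile is invalid.
; A GetGameMode macro handles the cast for GetGrid, printing an error on failure.
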(event EventBeginPlay
  (bind _grid (CallFunction|GetGrid))
  (bind _output_get (Variables|Default|SetGrid _grid))
  (if (Utilities|IsValid _output_get)
    (bind (_valid_ _row _column) (Default|LocationtoTile (Variables|Default|GetGrid) (Transformation|GetActorLocation)))
    (if _valid_
      (bind _location (Default|TiletoLocation (Variables|Default|GetGrid) _row _column))
      (Transformation|SetActorLocation _location false true)
      (else
        (Actor|DestroyActor :!label _label)))
    (else
      (goto _label))))

(fn ConstructionScript
  (bind _grid (CallFunction|GetGrid))
  (bind _output_get (Variables|Default|SetGrid _grid))
  (if (Utilities|IsValid _output_get)
    (bind (_valid_ _row _column) (Default|LocationtoTile (Variables|Default|GetGrid) (Transformation|GetActorLocation)))
    (if _valid_
      (bind _location (Default|TiletoLocation (Variables|Default|GetGrid) _row _column))
      (Transformation|SetActorLocation _location false true))
    (else
      (Development|PrintString "Failed to set gamemode"))))

(fn GetGrid
  (bind _gamemode (Utilities|GetGameMode)
    (:_Exec
      (bind _grid (Default|GetGrid _gamemode))
      (return _grid))))