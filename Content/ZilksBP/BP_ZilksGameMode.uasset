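; Game mode for the Zilks grid game that holds the level's grid reference and assigns joining players to teams.
; On BeginPlay it finds the first BP_ZilksGrid in the world and caches it, exposing it through GetGrid.
; On PostLogin it increments a player index and, after a short delay, tags the player's grid character Right or Left by alternating parity.
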(event EventBeginPlay
  (bind _returnvalue (CallFunction|SetGrid))
  (if _returnvalue
    (Development|PrintString "GAMEMODE - Grid set" true true "(R=0.000000,G=1.000000,B=0.140301,A=1.000000)")
    (else
      (Development|PrintString "GAMEMODE - Grid NOT set" true true "(R=1.000000,G=0.009182,B=0.000000,A=1.000000)"))))

(event EventTick
  (params (DeltaSeconds :type Float%20%28single-precision%29)))

(event EventPostLogin
  (params (NewPlayer :type Player%20Controller%20Object%20Reference))
  (bind _asbp_zilks_player_controller (Utilities|Casting|CastToBP_ZilksPlayerController NewPlayer))
  (bind _result (Math|Integer|IncrementInt (Variables|Default|GetPlayerIndex))
    (:%20%20
      (Utilities|FlowControl|Delay 0.2) ; TODO
      (bind _asbp_zilks_grid_character (Utilities|Casting|CastToBP_ZilksGridCharacter (Pawn|GetControlledPawn _asbp_zilks_player_controller)))
      (if (== (Math|Integer|%(Integer) _result 2) 0)
        (Variables|/Game/ZilksBP/BP_ZilksGridCharacter.BP_ZilksGridCharacter_C|SetTeamTag _asbp_zilks_grid_character "(TagName=\"Team.RightTeam\")")
        (Development|PrintString "set team right")
        (else
          (Variables|/Game/ZilksBP/BP_ZilksGridCharacter.BP_ZilksGridCharacter_C|SetTeamTag _asbp_zilks_grid_character "(TagName=\"Team.LeftTeam\")")
          (Development|PrintString "set team left"))))))

(fn ConstructionScript)

(fn SetGrid
  (bind _outactors (Actor|GetAllActorsOfClass "/Game/ZilksBP/BP_ZilksGrid.BP_ZilksGrid_C"))
  (if (Utilities|Array|IsValidIndex _outactors)
    (Variables|Default|SetGrid (Utilities|Array|Get(acopy) _outactors))
    (Development|PrintText "ZilksGameModeNew: valid Grid" true true "(R=0.000000,G=1.000000,B=0.000000,A=1.000000)")
    (return (Utilities|Array|IsValidIndex _outactors))
    (else
      (Development|PrintText "ZilksGameModeNew: invalid Grid" true true "(R=1.000000,G=0.000000,B=0.000000,A=1.000000)")
      (return false))))

(fn GetGrid
  (return (Variables|Default|GetGrid)))