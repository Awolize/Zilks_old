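; ZilksCharacterBP is a character Blueprint that turns the mouse cursor position into a selected tile on the game's grid.
; BeginPlay caches the Grid obtained from BP_ZilksGameMode through a GetGameMode cast macro.
; Each Tick traces under the cursor on the Visibility channel, aligns CursorToWorld to the hit point and normal, and converts that location to a tile.
; It passes the row and column to ZilksPlayerControllerBP, or -1 for both when nothing is hit.
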(event EventTick
  (params (DeltaSeconds :type Float%20%28single-precision%29))
  (CallFunction|UpdateCursorPosition))

(event EventBeginPlay
  (bind _grid (CallFunction|GetGrid))
  (Variables|Private|SetGrid _grid))

(fn ConstructionScript)

(fn UpdateCursorPosition
  (bind _returnvalue (Game|GetPlayerController 0))
  (bind (_hitresult _returnvalue_2) (Game|Player|GetHitResultUnderCursorbyChannel _returnvalue "TraceTypeQuery1" true))
  (bind (_bblockinghit _binitialoverlap _time _distance _location _impactpoint _normal _impactnormal) (Collision|BreakHitResult _hitresult))
  (if _returnvalue_2
    (bind _output_get (LocalVariables|SetHitLocation _location))
    (Transformation|SetWorldLocationAndRotation (Variables|Default|GetCursorToWorld) _output_get (Math|Rotator|MakeRotationfromAxes _impactnormal "0, 0, 0" "0, 0, 0") false false)
    (bind (_valid_ _row _column) (Default|LocationtoTile (Variables|Private|GetGrid) (LocalVariables|GetHitLocation)))
    (bind _aszilks_player_controller_bp (Utilities|Casting|CastToZilksPlayerControllerBP (Game|GetPlayerController 0)))
    (Default|SetSelectedTile _aszilks_player_controller_bp _row _column)
    (else
      (bind _aszilks_player_controller_bp_2 (Utilities|Casting|CastToZilksPlayerControllerBP (Game|GetPlayerController 0)))
      (Default|SetSelectedTile _aszilks_player_controller_bp_2 -1 -1))))

(fn GetGrid
  (bind _gamemode (Utilities|GetGameMode)
    (:_Exec
      (bind _grid (Default|GetGrid _gamemode))
      (return _grid))))